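; BP_Explosion_Actor is an explosion actor that knocks back and damages nearby characters as soon as it spawns.
; On BeginPlay it sphere-traces for objects within Radius, with debug drawing on, and launches each hit Character against the impact normal with distance falloff and a fixed upward boost.
; Each launched Character also takes damage through BPC_Health.
; The actor destroys itself only when the trace hits something.
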(event EventBeginPlay
  (bind _returnvalue (Transformation|GetActorLocation))
  (bind (_outhits _returnvalue_2) (Collision|MultiSphereTraceForObjects _returnvalue _returnvalue (Variables|Default|GetRadius) (Utilities|Array|MakeArray "ObjectTypeQuery3" "ObjectTypeQuery8") false 0 "ForDuration"))
  (if _returnvalue_2
    (for _array_element _outhits
      (bind _ascharacter (Utilities|Casting|CastToCharacter (.HitActor (Collision|BreakHitResult _array_element))))
      (Character|LaunchCharacter _ascharacter (+ (* (* (.ImpactNormal (Collision|BreakHitResult _array_element)) -1.0) (* (- 1.0 (/ (Math|Vector|VectorLength (- (Transformation|GetActorLocation) (.Location (Collision|BreakHitResult _array_element)))) (Variables|Default|GetRadius))) (Variables|Default|GetExplosion%20Max%20Knockback))) "0.000000,0.000000,500.000000") true true)
      (Default|TakeDamage (Actor|GetComponentbyClass (.HitActor (Collision|BreakHitResult _array_element)) "/Game/Player/Components/BPC_Health.BPC_Health_C") 1))
    (Actor|DestroyActor)))

(fn ConstructionScript)