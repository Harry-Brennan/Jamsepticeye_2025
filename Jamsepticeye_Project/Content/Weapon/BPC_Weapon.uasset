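; Weapon component for players and enemies that handles firing, cooldown, ammo and reloading.
; Loads stats from separate player or enemy data tables, chosen by the owner's interface.
; Firing switches on weapon type, activating pooled projectiles for straight, scattered, spread or explosive shots, while Sniper only runs a sphere trace without applying damage.
; Empty ammo triggers a timed refill, except that one player upgrade branch deals area damage without refilling.
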(event Custom|Cooldown%20Handler
  (params (Cooldown%20Duration :type Float%20%28double-precision%29))
  (Utilities|FlowControl|Delay Cooldown%20Duration)
  (Variables|Default|SetCan%20Shoot true))

(event Custom|Reload
  (bind _returnvalue (Components|GetOwner))
  (bind _returnvalue_2 (Transformation|GetActorLocation _returnvalue))
  (if (not (Variables|Default|GetReloading))
    (Variables|Default|SetReloading true)
    (Variables|Default|SetCan%20Shoot false)
    (Default|CallReloadMessage (Variables|WeaponInfo|GetReload%20Time))
    (if (Utilities|DoesObjectImplementInterface (Components|GetOwner) "/Game/Player/BPI_Player.BPI_Player_C")
      (bind _asbp_game_instance (Utilities|Casting|CastToBP_Game_Instance (Game|GetGameInstance)))
      (if (Utilities|Array|ContainsItem (Variables|/Game/Core/Instances/BP_Game_Instance.BP_Game_Instance_C|GetCurrent%20Player%20Upgrades _asbp_game_instance) "NewEnumerator7")
        (bind (_outhits _returnvalue_3) (Collision|MultiSphereTraceForObjects _returnvalue_2 _returnvalue_2 256.0 (Utilities|Array|MakeArray "ObjectTypeQuery8") false 0 "None"))
        (if _returnvalue_3
          (for _array_element _outhits
            (Default|TakeDamage (Actor|GetComponentbyClass (.HitActor (Collision|BreakHitResult _array_element)) "/Game/Player/Components/BPC_Health.BPC_Health_C") 1)))
        (else
          (Utilities|FlowControl|Delay (Variables|WeaponInfo|GetReload%20Time) :!label _label)
          (bind _output_get (Variables|Default|SetCurrent%20Ammo (Variables|WeaponInfo|GetMax%20Ammo)))
          (Default|CallAmmoUpdated _output_get)
          (Variables|Default|SetCan%20Shoot true)
          (Variables|Default|SetReloading false)))
      (else
        (goto _label)))))

(event EventBeginPlay
  (bind _returnvalue (Actor|GetActorOfClass "/Game/Weapon/BP_Projectile_Pooler.BP_Projectile_Pooler_C"))
  (Variables|Default|SetProjectile%20Pooler _returnvalue)
  (bind _ascharacter (Utilities|Casting|CastToCharacter (Components|GetOwner)))
  (Variables|Default|SetAs%20Character _ascharacter)
  (CallFunction|SetWeaponInfo (Variables|Default|GetEquipped%20Weapon)))

(event EventTick
  (params (DeltaSeconds :type Float%20%28single-precision%29)))

(fn FireEquippedWeapon
  (params (Shoot%20Loc :type Vector) (Shoot%20Rot :type Rotator))
  (if (and (not (<= (Variables|Default|GetCurrent%20Ammo) 0)) (Variables|Default|GetCan%20Shoot))
    (Variables|Default|SetCan%20Shoot false)
    (Utilities|FlowControl|Sequence
      (:then_0
        (switch Utilities|FlowControl|Switch|SwitchonEnum_Weapons (Variables|Default|GetEquipped%20Weapon)
          (:NewEnumerator0
            (|Pistol :!label _label))
          (:NewEnumerator1
            (|Shotgun))
          (:NewEnumerator2
            (|Sniper))
          (:NewEnumerator3
            (goto _label))
          (:NewEnumerator4
            (|Spread))
          (:NewEnumerator5
            (Default|ActivateNextProjectile (Variables|Default|GetProjectile%20Pooler) (+ (* (Math|Vector|GetForwardVector Shoot%20Rot) (* 1e+02 (Variables|Default|GetProjectile%20Scale))) (+ Shoot%20Loc (Math|Vector|MakeVector 0.0 0.0 (* (- (Variables|Default|GetProjectile%20Scale) 1.0) 25.0)))) Shoot%20Rot (Variables|WeaponInfo|GetProjectile%20Speed) (Variables|WeaponInfo|GetProjectile%20Lifespan) true 5e+02 (Variables|Default|GetProjectile%20Scale) (Utilities|DoesObjectImplementInterface (Components|GetOwner) "/Game/Player/BPI_Player.BPI_Player_C")))))
      (:then_1
        (CallFunction|CooldownHandler (* (Variables|WeaponInfo|GetCooldown%20Duration) 0.99))
        (CallFunction|ReduceAmmo)
        (if (== (Game|GetPlayerCharacter 0) (Components|GetOwner))
          (CameraShakes|StartCameraShake (Game|GetPlayerCameraManager 0) "/Game/Weapon/BP_Shoot_CS.BP_Shoot_CS_C" 0.5 "CameraLocal" "0, 0, 0"))))
    (elif (<= (Variables|Default|GetCurrent%20Ammo) 0)
      (CallFunction|Reload))))

(fn SetWeaponInfo
  (params (Selected%20Weapon :type Enum_Weapons%20Enum :default "NewEnumerator0"))
  (if (Utilities|DoesObjectImplementInterface (Components|GetOwner) "/Game/Enemies/BPI_Enemy_Main.BPI_Enemy_Main_C")
    (bind _returnvalue (Utilities|GetDataTableRow "/Game/Weapon/DT_Enemy_Weapons.DT_Enemy_Weapons" (Utilities|String|StringToName (Utilities|String|EnumtoString Selected%20Weapon)))
      (:then
        (Variables|Default|SetEquipped%20Weapon (.Enum (Utilities|Struct|BreakStruct_Weapon _returnvalue)))
        (Variables|WeaponInfo|SetProjectile%20Speed (.ProjectileSpeed (Utilities|Struct|BreakStruct_Weapon _returnvalue)))
        (Variables|WeaponInfo|SetCooldown%20Duration (.Cooldown (Utilities|Struct|BreakStruct_Weapon _returnvalue)))
        (Variables|WeaponInfo|SetProjectile%20Lifespan (.Lifespan (Utilities|Struct|BreakStruct_Weapon _returnvalue)))
        (bind _output_get (Variables|WeaponInfo|SetMax%20Ammo (.MaxAmmo (Utilities|Struct|BreakStruct_Weapon _returnvalue))))
        (bind _output_get_2 (Variables|Default|SetCurrent%20Ammo _output_get))
        (Variables|WeaponInfo|SetReload%20Time (.ReloadTime (Utilities|Struct|BreakStruct_Weapon _returnvalue)))
        (Variables|Default|SetProjectile%20Scale (.ProjectileScale (Utilities|Struct|BreakStruct_Weapon _returnvalue)))
        (Default|CallWeaponInfoUpdated (.Enum (Utilities|Struct|BreakStruct_Weapon _returnvalue)))
        (Default|CallAmmoUpdated _output_get_2)))
    (else
      (bind _returnvalue_2 (Utilities|GetDataTableRow "/Game/Weapon/DT_Weapons.DT_Weapons" (Utilities|String|StringToName (Utilities|String|EnumtoString Selected%20Weapon)))
        (:then
          (Variables|Default|SetEquipped%20Weapon (.Enum (Utilities|Struct|BreakStruct_Weapon _returnvalue_2)))
          (Variables|WeaponInfo|SetProjectile%20Speed (.ProjectileSpeed (Utilities|Struct|BreakStruct_Weapon _returnvalue_2)))
          (Variables|WeaponInfo|SetCooldown%20Duration (.Cooldown (Utilities|Struct|BreakStruct_Weapon _returnvalue_2)))
          (Variables|WeaponInfo|SetProjectile%20Lifespan (.Lifespan (Utilities|Struct|BreakStruct_Weapon _returnvalue_2)))
          (bind _output_get_3 (Variables|WeaponInfo|SetMax%20Ammo (.MaxAmmo (Utilities|Struct|BreakStruct_Weapon _returnvalue_2))))
          (bind _output_get_4 (Variables|Default|SetCurrent%20Ammo _output_get_3))
          (Variables|WeaponInfo|SetReload%20Time (.ReloadTime (Utilities|Struct|BreakStruct_Weapon _returnvalue_2)))
          (Variables|Default|SetProjectile%20Scale (.ProjectileScale (Utilities|Struct|BreakStruct_Weapon _returnvalue_2)))
          (Default|CallWeaponInfoUpdated (.Enum (Utilities|Struct|BreakStruct_Weapon _returnvalue_2)))
          (Default|CallAmmoUpdated _output_get_4))))))

(fn ReduceAmmo
  (bind _output_get (Variables|Default|SetCurrent%20Ammo (- (Variables|Default|GetCurrent%20Ammo) 1)))
  (Default|CallAmmoUpdated _output_get))