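; Reusable fire-orb projectile for player and enemy shots, switched on and off via Activate/Deactivate rather than spawned and destroyed.
; Activation sets transform, speed, Pawn collision response and Niagara look, then starts a lifespan timer.
; Overlaps optionally spawn an explosion, damage BPC_Health owners or leave a fading, randomized blood decal, then deactivate.
; A riot-shield match on enemies skips damage and decals, deactivating only explosive shots.
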(event OnComponentBeginOverlap(Sphere)
  (params (OverlappedComponent :type Primitive%20Component%20Object%20Reference) (OtherActor :type Actor%20Object%20Reference) (OtherComp :type Primitive%20Component%20Object%20Reference) (OtherBodyIndex :type Integer) (bFromSweep :type Boolean) (SweepResult :type Hit%20Result%20Structure%20%28by%20ref%29))
  (bind (_bblockinghit _binitialoverlap _time _distance _location _impactpoint _normal _impactnormal) (Collision|BreakHitResult SweepResult))
  (bind _returnvalue (Actor|GetComponentbyClass OtherActor "/Game/Player/Components/BPC_Health.BPC_Health_C"))
  (if (Utilities|DoesObjectImplementInterface OtherActor "/Game/Enemies/BPI_Enemy_Main.BPI_Enemy_Main_C")
    (bind _riot_shield (Class|BPIEnemyMain|GetRiotShield(Message) OtherActor))
    (if (== _riot_shield OverlappedComponent)
      (if (Variables|Default|GetShould%20Explode)
        (Game|SpawnActorfromClass "/Game/Weapon/BP_Explosion_Actor.BP_Explosion_Actor_C" (Math|Transform|MakeTransform (Transformation|GetActorLocation) "0, 0, 0" "1.000000,1.000000,1.000000") "Undefined" "MultiplyWithRoot" 0 0)
        (CallFunction|DeactivateProjectile))
      (else
        (if (Variables|Default|GetShould%20Explode) :!label _label
          (Game|SpawnActorfromClass "/Game/Weapon/BP_Explosion_Actor.BP_Explosion_Actor_C" (Math|Transform|MakeTransform (Transformation|GetActorLocation) "0, 0, 0" "1.000000,1.000000,1.000000") "Undefined" "MultiplyWithRoot" 0 0))
        (Utilities|IsValid _returnvalue
          (:Is%20Valid
            (Default|TakeDamage _returnvalue 1)
            (CallFunction|DeactivateProjectile))
          (:Is%20Not%20Valid
            (CallFunction|DeactivateProjectile)
            (bind _returnvalue_2 (Rendering|Decal|SpawnDecalatLocation "/Game/VFX/Blood_Splatter/Materials/MI_Blood_Decal.MI_Blood_Decal" "32.000000,32.000000,32.000000" _location (Math|Conversions|RotationFromXVector (* _impactnormal -1.0)) 5.0))
            (Rendering|Components|Decal|SetFadeOut _returnvalue_2 3.0 1.0 true)
            (bind _returnvalue_3 (Rendering|Material|CreateDynamicMaterialInstance _returnvalue_2 :!class /Script/Engine.DecalComponent))
            (Rendering|Material|SetScalarParameterValue _returnvalue_3 "Radius" (Math|Random|RandomFloatinRange 5.0 15.0) :!class /Script/Engine.MaterialInstanceDynamic)))))
    (else
      (goto _label))))

(event Custom|Deactivate%20Projectile
  (Rendering|SetActorHiddenInGame true)
  (Collision|SetActorEnableCollision false)
  (Components|Activation|Deactivate (Variables|Default|GetNiagara)))

(event Custom|Activate%20Projectile
  (params (Loc :type Vector) (Rot :type Rotator) (Speed :type Float%20%28double-precision%29) (Lifespan :type Float%20%28double-precision%29) (Should%20Explode :type Boolean) (Explosion%20Radius :type Float%20%28double-precision%29) (Scale :type Float%20%28double-precision%29) (IsPlayer? :type Boolean))
  (Collision|SetCollisionResponsetoChannel (Variables|Default|GetSphere) "ECC_Pawn" (select IsPlayer? "ECR_Ignore" "ECR_Overlap"))
  (Transformation|SetActorScale3D (Math|Vector|MakeVector Scale Scale Scale))
  (Class|NiagaraComponent|SetAsset (Variables|Default|GetNiagara) (select IsPlayer? "/Game/VFX/Projectiles/NS_Fire_Orb_Player.NS_Fire_Orb_Player" "/Game/VFX/Projectiles/NS_Fire_Orb.NS_Fire_Orb") true)
  (Utilities|Time|ClearandInvalidateTimerbyHandle (Variables|Default|GetLifespan%20Timer))
  (Transformation|SetActorLocationAndRotation Loc Rot)
  (bind _output_get (Variables|/Script/Engine.ProjectileMovementComponent|SetInitialSpeed (Variables|Default|GetProjectileMovement) Speed))
  (bind _output_get_2 (Variables|/Script/Engine.ProjectileMovementComponent|SetMaxSpeed (Variables|Default|GetProjectileMovement) _output_get))
  (Variables|/Script/Engine.MovementComponent|SetVelocity (Variables|Default|GetProjectileMovement) (* _output_get_2 (Math|Vector|GetForwardVector (Transformation|GetActorRotation))))
  (Rendering|SetActorHiddenInGame false)
  (Collision|SetActorEnableCollision true)
  (Variables|Default|SetLifespan Lifespan)
  (Variables|Default|SetSpeed Speed)
  (Variables|Default|SetShould%20Explode Should%20Explode)
  (Variables|Default|SetExplode%20Radius Explosion%20Radius)
  (Components|Movement|SetUpdatedComponent (Variables|Default|GetProjectileMovement) (Variables|Default|GetSphere))
  (Components|Activation|Activate (Variables|Default|GetNiagara) false)
  (bind _returnvalue (Utilities|Time|SetTimerbyFunctionName 0 "Deactivate Projectile" (Variables|Default|GetLifespan)))
  (Variables|Default|SetLifespan%20Timer _returnvalue))

(fn ConstructionScript
  (Variables|/Script/Engine.ProjectileMovementComponent|SetInitialSpeed (Variables|Default|GetProjectileMovement) (Variables|Default|GetSpeed)))