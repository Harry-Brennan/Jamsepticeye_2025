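; BP_Projectile_Pooler is an object pool that supplies reusable projectiles for weapon fire.
; On BeginPlay it pre-spawns a fixed batch of BP_Projectile actors, hidden and with collision disabled, and stores them in an array.
; ActivateNextProjectile passes the shot parameters to the projectile at the current index, then advances that index round-robin, wrapping to the start without checking whether that projectile is still active.
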(event Custom|Activate%20Next%20Projectile
  (params (Loc :type Vector) (Rot :type Rotator) (Speed :type Float%20%28double-precision%29) (Lifespan :type Float%20%28double-precision%29) (Should%20Explode :type Boolean) (Explosion%20Radius :type Float%20%28double-precision%29) (Scale :type Float%20%28double-precision%29) (IsPlayer? :type Boolean))
  (Default|ActivateProjectile (Utilities|Array|Get(acopy) (Variables|Default|GetProjectile%20Pool) (Variables|Default|GetCurrent%20Projectile%20Pool%20Index)) Loc Rot Speed Lifespan Should%20Explode Explosion%20Radius Scale IsPlayer?)
  (if (> (+ (Variables|Default|GetCurrent%20Projectile%20Pool%20Index) 1) (Utilities|Array|LastIndex (Variables|Default|GetProjectile%20Pool)))
    (Variables|Default|SetCurrent%20Projectile%20Pool%20Index 0)
    (else
      (Math|Integer|IncrementInt (Variables|Default|GetCurrent%20Projectile%20Pool%20Index)))))

(event EventBeginPlay
  (for _index (range 0 30)
    (bind _returnvalue (Game|SpawnActorfromClass "/Game/Weapon/BP_Projectile.BP_Projectile_C" (Math|Transform|MakeTransform "0, 0, 0" "0, 0, 0" "1.000000,1.000000,1.000000") "AlwaysSpawn" "MultiplyWithRoot" 0 0.0 0.0 0))
    (Utilities|Array|Add (Variables|Default|GetProjectile%20Pool) _returnvalue)
    (Collision|SetActorEnableCollision _returnvalue false)
    (Rendering|SetActorHiddenInGame _returnvalue true)))

(fn ConstructionScript)