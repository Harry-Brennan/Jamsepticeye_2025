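; Enemy director that spawns enemies at random spawn points under a point budget, with budget and spawn frequency scaled by rooms cleared.
; It pre-spawns a BP_Enemy pool and activates members round-robin on a randomized timer, using cost-tiered random types and DT_Enemy_Info data.
; Enemy deaths refund points, restart spawning from zero points, update score and combo, and reset player health every ten kills with a specific upgrade.
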(event Custom|Stop%20Spawning%20Loop
  (Utilities|Time|ClearandInvalidateTimerbyHandle (Variables|Default|GetSpawn%20Enemy%20Timer)))

(event Custom|Start%20Spawning%20Loop
  (bind _returnvalue (Utilities|Time|SetTimerbyFunctionName 0 "Spawn Enemy" (Math|Random|RandomFloatinRange (Variables|Default|GetSpawn%20Freq%20Min) (Variables|Default|GetSpawn%20Freq%20Max))))
  (Variables|Default|SetSpawn%20Enemy%20Timer _returnvalue))

(event EventBeginPlay
  (bind _outactors (Actor|GetAllActorsOfClass "/Game/Enemies/BP_Enemy_Spawn_Point.BP_Enemy_Spawn_Point_C"))
  (Variables|Default|SetEnemy%20Spawn%20Points _outactors)
  (bind _asbp_game_instance (Utilities|Casting|CastToBP_Game_Instance (Game|GetGameInstance)))
  (Variables|Default|SetMax%20Points (Math|Float|Truncate (Math|Float|MapRangeClamped (Math|Conversions|ToFloat(Integer) (Variables|/Game/Core/Instances/BP_Game_Instance.BP_Game_Instance_C|GetRooms%20Cleared _asbp_game_instance)) 1.0 4.0 25.0 1e+02)))
  (Variables|Default|SetSpawn%20Freq%20Max (Math|Float|MapRangeClamped (Math|Conversions|ToFloat(Integer) (Variables|/Game/Core/Instances/BP_Game_Instance.BP_Game_Instance_C|GetRooms%20Cleared _asbp_game_instance)) 1.0 4.0 3.5 1.0))
  (Variables|Default|SetSpawn%20Freq%20Min (Math|Float|MapRangeClamped (Math|Conversions|ToFloat(Integer) (Variables|/Game/Core/Instances/BP_Game_Instance.BP_Game_Instance_C|GetRooms%20Cleared _asbp_game_instance)) 1.0 4.0 2.0 0.5))
  (Variables|Default|SetCurrent%20Points (Variables|Default|GetMax%20Points))
  (for _index (range 0 (Variables|Default|GetNum%20Enemies%20to%20Pool))
    (bind _returnvalue (Game|SpawnActorfromClass :Class "/Game/Enemies/BP_Enemy.BP_Enemy_C" :CollisionHandlingOverride "Undefined" :TransformScaleMethod "MultiplyWithRoot" :Instigator 0))
    (EventDispatchers|BindEventtoEnemyDeath _returnvalue (EventDispatchers|CreateEvent :!event EnemyDeath))
    (Utilities|Array|Add (Variables|Default|GetEnemy%20Pool) _returnvalue)))

(fn ConstructionScript)

(fn SpawnEnemy
  (Development|PrintString "SPAWN ENEMY FUNC CALLED")
  (LocalVariables|SetNum%20Enemies%20to%20Spawn (CallFunction|CalcNumEnemiestoSpawn))
  (bind _enemy_type_to_spawn (CallFunction|CalcEnemytoSpawn :!label _label))
  (bind (_can _points_used) (CallFunction|CheckCanSpawnEnemyType _enemy_type_to_spawn))
  (if _can
    (Variables|Default|SetCurrent%20Points (- (Variables|Default|GetCurrent%20Points) _points_used))
    (bind _returnvalue (Utilities|GetDataTableRow "/Game/Enemies/DT_Enemy_Info.DT_Enemy_Info" (Utilities|String|StringToName (Utilities|String|EnumtoString _enemy_type_to_spawn)))
      (:then
        (bind _output_get (LocalVariables|SetSpawn%20Point (.OutItem (Utilities|Array|Random (Variables|Default|GetEnemy%20Spawn%20Points)))))
        (Default|ActivateEnemy (Utilities|Array|Get(acopy) (Variables|Default|GetEnemy%20Pool) (Variables|Default|GetCurrent%20Enemy%20Pool%20Index)) _returnvalue (Transformation|GetActorLocation _output_get))
        (Development|PrintString (Utilities|String|Append (Utilities|GetDisplayName _output_get) " - " (Utilities|String|ToString(Name) (Utilities|String|StringToName (Utilities|String|EnumtoString _enemy_type_to_spawn)))) true true "(R=0.000000,G=0.660000,B=1.000000,A=1.000000)" 1e+02)
        (if (> (+ (Variables|Default|GetCurrent%20Enemy%20Pool%20Index) 1) (Utilities|Array|LastIndex (Variables|Default|GetEnemy%20Pool)))
          (Variables|Default|SetCurrent%20Enemy%20Pool%20Index 0)
          (else
            (Math|Integer|IncrementInt (Variables|Default|GetCurrent%20Enemy%20Pool%20Index)
              (:%20%20
                _))))
        (Math|Integer|IncrementInt (LocalVariables|GetEnemies%20Spawned)
          (:%20%20
            (if (== (LocalVariables|GetEnemies%20Spawned) (LocalVariables|GetNum%20Enemies%20to%20Spawn))
              (bind _returnvalue_2 (Utilities|Time|SetTimerbyFunctionName 0 "Spawn Enemy" (Math|Random|RandomFloatinRange (Variables|Default|GetSpawn%20Freq%20Min) (Variables|Default|GetSpawn%20Freq%20Max))))
              (Variables|Default|SetSpawn%20Enemy%20Timer _returnvalue_2)
              (else
                (goto _label)))))))
    (elif (not (< (Variables|Default|GetCurrent%20Points) 0))
      (goto _label))))

(fn EnemyDeath
  (params (Enemy%20Cost :type Integer) (Enemy%20Score :type Integer))
  (bind _returnvalue (Game|GetPlayerCharacter 0))
  (bind _returnvalue_2 (Actor|GetComponentbyClass _returnvalue "/Game/Player/Components/BPC_Health.BPC_Health_C"))
  (if (== (Variables|Default|GetCurrent%20Points) 0)
    (bind _returnvalue_3 (Utilities|Time|SetTimerbyFunctionName 0 "Spawn Enemy" (Math|Random|RandomFloatinRange (Variables|Default|GetSpawn%20Freq%20Min) (Variables|Default|GetSpawn%20Freq%20Max))))
    (Variables|Default|SetSpawn%20Enemy%20Timer _returnvalue_3))
  (Variables|Default|SetCurrent%20Points (Math|Integer|Clamp(Integer) (+ (Variables|Default|GetCurrent%20Points) Enemy%20Cost) 0 (Variables|Default|GetMax%20Points)))
  (bind _asbp_in_game (Utilities|Casting|CastToBP_In_Game (Game|GetGameMode)))
  (Default|IncrementCombo _asbp_in_game)
  (Default|UpdateScore _asbp_in_game Enemy%20Score)
  (bind _asbp_game_instance (Utilities|Casting|CastToBP_Game_Instance (Game|GetGameInstance)))
  (if (Utilities|Array|ContainsItem (Variables|/Game/Core/Instances/BP_Game_Instance.BP_Game_Instance_C|GetCurrent%20Player%20Upgrades _asbp_game_instance) "NewEnumerator8")
    (bind _result (Math|Integer|IncrementInt (Variables|Default|GetEnemy%20Kill%20Check))
      (:%20%20
        (if (>= _result 10)
          (Variables|/Game/Player/Components/BPC_Health.BPC_Health_C|SetHealth%20Points _returnvalue_2 2)
          (Default|CallPlayerResetHealth _returnvalue_2)
          (Variables|Default|SetEnemy%20Kill%20Check 0))))))

(fn CalcEnemytoSpawn
  (bind _returnvalue (Math|Random|RandomIntegerinRange 0 99))
  (if (< _returnvalue 40)
    (return (.OutItem (Utilities|Array|Random (Variables|Default|GetCheap%20Enemies))))
    (elif (and (< _returnvalue 60) (> _returnvalue 40))
      (return (.OutItem (Utilities|Array|Random (Variables|Default|GetMedium%20Enemies))))
      (elif (and (< _returnvalue 75) (> _returnvalue 60))
        (return (.OutItem (Utilities|Array|Random (Variables|Default|GetExpensive%20Enemies))))
        (elif (> _returnvalue 75)
          (return (.OutItem (Utilities|Array|Random (Variables|Default|GetExtreme%20Enemies))))
          (else
            (return "NewEnumerator0")))))))

(fn CheckCanSpawnEnemyType
  (params (Enemy%20Type :type Enum_Enemy_Type%20Enum :default "NewEnumerator0"))
  (bind _returnvalue (Utilities|GetDataTableRow "/Game/Enemies/DT_Enemy_Info.DT_Enemy_Info" (Utilities|String|StringToName (Utilities|String|EnumtoString Enemy%20Type)))
    (:then
      (return (> (- (Variables|Default|GetCurrent%20Points) (.SpawnCost (Utilities|Struct|BreakStruct_Enemy_Info _returnvalue))) -1) (.SpawnCost (Utilities|Struct|BreakStruct_Enemy_Info _returnvalue))))
    (:RowNotFound
      (return false 0))))

(fn CalcNumEnemiestoSpawn
  (return (Math|Random|RandomIntegerinRange 2 3)))