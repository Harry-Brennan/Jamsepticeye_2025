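; Pooled enemy character that is parked hidden at an inactive transform, then configured from EnemyInfo on activation and returned on death.
; Enemy type selects riot shield, single-ally magic shield linking or possession-immunity aura, the latter two using timed sphere traces, or an explosion on death.
; Activation starts the AIC_Enemy controller and arms BPC_Weapon.
; Attacks either fire at the player or play a timeline-stretched melee telegraph ending in a damage trace.
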(event OnComponentBeginOverlap(RiotShield)
  (params (OverlappedComponent :type Primitive%20Component%20Object%20Reference) (OtherActor :type Actor%20Object%20Reference) (OtherComp :type Primitive%20Component%20Object%20Reference) (OtherBodyIndex :type Integer) (bFromSweep :type Boolean) (SweepResult :type Hit%20Result%20Structure%20%28by%20ref%29))
  (bind _asbp_projectile (Utilities|Casting|CastToBP_Projectile OtherActor))
  (Default|DeactivateProjectile _asbp_projectile))

(event Custom|Deactivate%20Riot%20Shield
  (bind _riot_shield (Variables|Default|GetRiot%20Shield))
  (Rendering|SetVisibility _riot_shield false false)
  (Collision|SetCollisionProfileName _riot_shield "NoCollision" true :!class /Script/Engine.PrimitiveComponent)
  (Collision|SetCollisionEnabled _riot_shield "NoCollision")
  (Variables|Default|SetRiot%20Shield%20Active false))

(event Custom|Activate%20Riot%20Shield
  (bind _riot_shield (Variables|Default|GetRiot%20Shield))
  (Rendering|SetVisibility _riot_shield true false)
  (Collision|SetCollisionProfileName _riot_shield "Riot_Shield_Active" true :!class /Script/Engine.PrimitiveComponent)
  (Collision|SetCollisionEnabled _riot_shield "QueryOnly")
  (Variables|Default|SetRiot%20Shield%20Active true))

(event Custom|Activate%20Possession%20Immunity
  (Variables|Default|SetPossession%20Immune true)
  (Rendering|SetVisibility (Variables|Default|GetPossession%20Immunity%20Indicator) true false))

(event Custom|Deactivate%20Possession%20Immunity
  (Variables|Default|SetPossession%20Immune false)
  (Rendering|SetVisibility (Variables|Default|GetPossession%20Immunity%20Indicator) false false))

(event Custom|Activate%20Possession%20Immunity%20AOE%20Loop
  (bind _returnvalue (Utilities|Time|SetTimerbyEvent (delegate Custom|Possession%20Immunity%20AOE%20Loop) 0.25 true)))

(event Custom|Possession%20Immunity%20AOE%20Loop
  (bind _returnvalue (Transformation|GetActorLocation))
  (bind _new_possession_immunity_affected_enemies (Variables|Default|GetNew%20Possession%20Immunity%20Affected%20Enemies))
  (bind (_outhits _returnvalue_2) (Collision|MultiSphereTraceForObjects _returnvalue _returnvalue 512.0 (Utilities|Array|MakeArray "ObjectTypeQuery8") false 0 "ForDuration"))
  (if _returnvalue_2
    (for _array_element _outhits
      (bind _asbp_enemy (Utilities|Casting|CastToBP_Enemy (.HitActor (Collision|BreakHitResult _array_element))))
      (if (Utilities|Array|ContainsItem (Variables|Default|GetPossession%20Immunity%20Affected%20Enemies) _asbp_enemy)
        _
        (else
          (Utilities|Array|Add (Variables|Default|GetPossession%20Immunity%20Affected%20Enemies) _asbp_enemy)
          (CallFunction|ActivatePossessionImmunity _asbp_enemy)))
      (Utilities|Array|Add (Variables|Default|GetNew%20Possession%20Immunity%20Affected%20Enemies) _asbp_enemy))
    (for _array_element_2 (Variables|Default|GetPossession%20Immunity%20Affected%20Enemies)
      (if (not (Utilities|Array|ContainsItem (Variables|Default|GetNew%20Possession%20Immunity%20Affected%20Enemies) _array_element_2))
        (CallFunction|DeactivatePossessionImmunity _array_element_2)))
    (Variables|Default|SetPossession%20Immunity%20Affected%20Enemies _new_possession_immunity_affected_enemies)
    (Utilities|Array|Clear _new_possession_immunity_affected_enemies)))

(event Custom|Deactivate%20Possession%20Immunity%20AOE%20Loop
  (Utilities|Time|ClearandInvalidateTimerbyHandle (stale Custom|Activate%20Possession%20Immunity%20AOE%20Loop _returnvalue)))

(event Custom|Update%20Enemy%20Info%20Associated
  (bind _enemy_info (Variables|Default|GetEnemy%20Info))
  (bind (_enemytype _attacks_ _enemyspeed _enemymaxhealth) (Utilities|Struct|BreakStruct_Enemy_Info _enemy_info))
  (Variables|/Game/Player/Components/BPC_Health.BPC_Health_C|SetHealth%20Points (Variables|Default|GetBPC_Health) _enemymaxhealth)
  (Variables|/Script/Engine.CharacterMovementComponent|SetMaxWalkSpeed (Variables|Character|GetCharacterMovement) _enemyspeed)
  (Variables|/Script/Engine.CharacterMovementComponent|SetRotationRate (Variables|Character|GetCharacterMovement) (Math|Rotator|SelectRotator "0.000000,240.000000,0.000000" "0.000000,360.000000,0.000000" (Utilities|Enum|Equal(Enum) (.EnemyType (Utilities|Struct|BreakStruct_Enemy_Info (Variables|Default|GetEnemy%20Info))) "NewEnumerator12"))))

(event Custom|Disable%20Magic%20Shield
  ;[0 0 0] Linker
  (Variables|Default|SetMagic%20Shielded false)
  (Variables|/Game/Player/Components/BPC_Health.BPC_Health_C|SetInvincible (Variables|Default|GetBPC_Health) false)
  (Rendering|SetVisibility (Variables|Default|GetShielded%20Indicator) false false))

(event Custom|Activate%20Magic%20Shield
  ;[0 0 0] Linker
  (Variables|Default|SetMagic%20Shielded true)
  (Variables|/Game/Player/Components/BPC_Health.BPC_Health_C|SetInvincible (Variables|Default|GetBPC_Health) true)
  (Rendering|SetVisibility (Variables|Default|GetShielded%20Indicator) true false))

(event Custom|Find%20Enemy%20to%20Shield%20Loop
  (bind _returnvalue (Transformation|GetActorLocation))
  ;[0 0 0] Linker
  (bind (_outhit _returnvalue_2) (Collision|SphereTraceForObjects _returnvalue _returnvalue 256.0 (Utilities|Array|MakeArray "ObjectTypeQuery8") false 0 "ForDuration"))
  (if _returnvalue_2
    (bind _asbp_enemy (Utilities|Casting|CastToBP_Enemy (.HitActor (Collision|BreakHitResult _outhit))))
    (Variables|Default|SetLinked%20Enemy _asbp_enemy)
    (CallFunction|ActivateMagicShield _asbp_enemy)
    (CallFunction|DeactivateFindEnemytoShieldLoop)))

(event Custom|Deactivate%20Find%20Enemy%20to%20Shield%20Loop
  ;[0 0 0] Linker
  (Utilities|Time|ClearandInvalidateTimerbyHandle (stale Custom|Activate%20Find%20Enemy%20to%20Shield%20Loop _returnvalue)))

(event Custom|Activate%20Find%20Enemy%20to%20Shield%20Loop
  ;[0 0 0] Linker
  (bind _returnvalue (Utilities|Time|SetTimerbyEvent (delegate Custom|Find%20Enemy%20to%20Shield%20Loop) 1.0 true)))

(event EventActivatePossessionIndicator
  (Rendering|SetVisibility (Variables|Default|GetPossession%20Indicator) true false))

(event EventDeactivatePossessionIndicator
  (Rendering|SetVisibility (Variables|Default|GetPossession%20Indicator) false false))

(event EventEnemyDeathEvent
  (bind _enemy_info (Variables|Default|GetEnemy%20Info))
  (bind (_enemytype _attacks_ _enemyspeed _enemymaxhealth _spawncost _weapon _scoreondeath) (Utilities|Struct|BreakStruct_Enemy_Info _enemy_info))
  (Default|CallEnemyDeath _spawncost _scoreondeath)
  (Game|SpawnActorfromClass "/Game/VFX/Bloodsplosion/BP_Bloodsplosion.BP_Bloodsplosion_C" (Math|Transform|MakeTransform (Transformation|GetActorLocation) "0, 0, 0" "1.000000,1.000000,1.000000") "Undefined" "MultiplyWithRoot" 0 0)
  (if (Utilities|Enum|Equal(Enum) (.EnemyType (Utilities|Struct|BreakStruct_Enemy_Info (Variables|Default|GetEnemy%20Info))) "NewEnumerator5")
    (Game|SpawnActorfromClass "/Game/Weapon/BP_Explosion.BP_Explosion_C" (Math|Transform|MakeTransform "0, 0, 0" "0, 0, 0" "1.000000,1.000000,1.000000") "Undefined" "MultiplyWithRoot" 0 5e+02 0))
  (CallFunction|DeactivateEnemy))

(event EventUpdateAttacking
  (params (Attacking :type Boolean) (Delay :type Float%20%28double-precision%29))
  (if (== Delay 0.0)
    (Utilities|FlowControl|Delay Delay))
  (Variables|Default|SetAttacking Attacking))

(event EventBeginPlay
  (bind _returnvalue (Actor|GetActorOfClass "/Game/Enemies/BP_Enemy_Inactive_Transform.BP_Enemy_Inactive_Transform_C"))
  (Variables|Default|SetInactive%20Transform _returnvalue)
  (if (Variables|Default|GetDummy?)
    (Rendering|SetActorHiddenInGame true)
    (Niagara|SpawnSystematLocation "/Game/VFX/NS_Enemy_Spawn.NS_Enemy_Spawn" (Transformation|GetActorLocation))
    (Utilities|FlowControl|Delay 1.0)
    (Rendering|SetActorHiddenInGame false)
    (else
      (CallFunction|DeactivateEnemy))))

(event EventDeactivateEnemy
  (bind _linked_enemy (Variables|Default|GetLinked%20Enemy))
  (Rendering|SetActorHiddenInGame true)
  (Transformation|SetActorLocation (Transformation|GetActorLocation (Variables|Default|GetInactive%20Transform)) false false)
  (CallFunction|DeactivatePossessionImmunityAOELoop)
  (CallFunction|DeactivateFindEnemytoShieldLoop)
  (Variables|/Script/Engine.PrimitiveComponent|SetbGenerateOverlapEvents (Variables|Collision|GetCapsuleComponent) false)
  (Utilities|IsValid _linked_enemy
    (:Is%20Valid
      (CallFunction|DisableMagicShield _linked_enemy))))

(event EventActivateEnemy
  (params (Enemy%20Info :type Struct%20Enemy%20Info%20Structure) (Location :type Vector :default "0, 0, 0"))
  (Variables|Default|SetEnemy%20Info Enemy%20Info)
  (Transformation|SetActorLocation Location false false)
  (CallFunction|UpdateEnemyInfoAssociated)
  (Niagara|SpawnSystematLocation "/Game/VFX/NS_Enemy_Spawn.NS_Enemy_Spawn" (Transformation|GetActorLocation))
  (Utilities|FlowControl|Delay 1.0)
  (Variables|/Script/Engine.PrimitiveComponent|SetbGenerateOverlapEvents (Variables|Collision|GetCapsuleComponent) true)
  (Variables|Default|SetPlayer%20Ref (Game|GetPlayerCharacter 0))
  (Default|SetWeaponInfo (Variables|Default|GetBPC_Weapon) (.Weapon (Utilities|Struct|BreakStruct_Enemy_Info (Variables|Default|GetEnemy%20Info))))
  (bind _asaic_enemy (Utilities|Casting|CastToAIC_Enemy (Pawn|GetController)))
  (Default|ActivateEnemyController _asaic_enemy)
  (Rendering|SetActorHiddenInGame false)
  (if (Utilities|Enum|Equal(Enum) (Utilities|Struct|BreakStruct_Enemy_Info (Variables|Default|GetEnemy%20Info)) "NewEnumerator12")
    (CallFunction|ActivateRiotShield)
    (Rendering|SetVisibility (Variables|Default|GetShielded%20Source%20Indicator) false false)
    (Rendering|SetVisibility (Variables|Default|GetPossession%20Immunity%20Source%20Indicator) false false)
    ;[0 0 0] Linker
    (CallFunction|DeactivatePossessionImmunityAOELoop)
    (else
      (CallFunction|DeactivateRiotShield)
      (Rendering|SetVisibility (Variables|Default|GetShielded%20Source%20Indicator) (Utilities|Enum|Equal(Enum) (Utilities|Struct|BreakStruct_Enemy_Info (Variables|Default|GetEnemy%20Info)) "NewEnumerator11") false)
      (if (Utilities|Enum|Equal(Enum) (Utilities|Struct|BreakStruct_Enemy_Info (Variables|Default|GetEnemy%20Info)) "NewEnumerator11")
        (CallFunction|ActivateFindEnemytoShieldLoop)
        (else
          (Rendering|SetVisibility (Variables|Default|GetPossession%20Immunity%20Source%20Indicator) (Utilities|Enum|Equal(Enum) (Utilities|Struct|BreakStruct_Enemy_Info (Variables|Default|GetEnemy%20Info)) "NewEnumerator10") false)
          (if (Utilities|Enum|Equal(Enum) (Utilities|Struct|BreakStruct_Enemy_Info (Variables|Default|GetEnemy%20Info)) "NewEnumerator10")
            (CallFunction|ActivatePossessionImmunityAOELoop)
            (else
              (CallFunction|DeactivatePossessionImmunityAOELoop))))))))

(event EventAttack
  (params (Ranged? :type Boolean))
  (bind _returnvalue (Transformation|GetActorLocation))
  (if Ranged?
    (Class|NiagaraComponent|SetAsset (Variables|Default|GetAttack%20Indicator) "/Game/VFX/NS_Enemy_Ranged_Charge.NS_Enemy_Ranged_Charge" true)
    (Components|Activation|Activate (Variables|Default|GetAttack%20Indicator) false)
    (CallFunction|UpdateAttacking true 0.0)
    (Default|FireEquippedWeapon (Actor|GetComponentbyClass "/Game/Weapon/BPC_Weapon.BPC_Weapon_C") (Transformation|GetActorLocation) (Math|Rotator|FindLookatRotation (Transformation|GetActorLocation) (Transformation|GetActorLocation (Game|GetPlayerCharacter 0))))
    (Utilities|FlowControl|Delay 0.1)
    (CallFunction|UpdateAttacking false 0.0)
    (else
      (Class|NiagaraComponent|SetAsset (Variables|Default|GetAttack%20Indicator) "/Game/VFX/NS_Enemy_Melee_Charged.NS_Enemy_Melee_Charged" true)
      (Components|Activation|Activate (Variables|Default|GetAttack%20Indicator) false)
      (CallFunction|UpdateAttacking true 0.0)
      (Rendering|Material|SetMaterial (Variables|Default|GetSM_Enemy_Melee_Indicator) 0 "/Game/Enemies/MI_Riot_Shield.MI_Riot_Shield")
      (Rendering|SetVisibility (Variables|Default|GetSM_Enemy_Melee_Indicator) true false)
      (Components|Timeline|SetPlayRate (Variables|Default|GetMelee%20Indicator%20Lengthen) (/ 1.0 0.25))
      (bind _alpha (Timeline|Melee%20Indicator%20Lengthen PlayFromStart)
        (:Update
          (Transformation|SetRelativeScale3D (Variables|Default|GetSM_Enemy_Melee_Indicator) (Math|Vector|MakeVector 0.3 0.7 (Math|Float|Lerp 0.05 2.0 _alpha))))
        (:Finished
          (Rendering|SetVisibility (Variables|Default|GetSM_Enemy_Melee_Indicator) false false)
          (bind (_outhit _returnvalue_2) (Collision|SphereTraceForObjects _returnvalue (+ (* (Math|Vector|GetForwardVector (Pawn|GetControlRotation :!class /Script/Engine.Pawn)) 2.5e+02) _returnvalue) 32.0 (Utilities|Array|MakeArray "ObjectTypeQuery3") false 0 "ForDuration"))
          (if _returnvalue_2
            (Default|TakeDamage (Actor|GetComponentbyClass (.HitActor (Collision|BreakHitResult _outhit)) "/Game/Player/Components/BPC_Health.BPC_Health_C") 1))
          (CallFunction|UpdateAttacking false 3.0))
        (:Flash
          (Rendering|Material|SetMaterial (Variables|Default|GetSM_Enemy_Melee_Indicator) 0 "/Game/Enemies/M_Enemy_Melee_Indicator_Flash.M_Enemy_Melee_Indicator_Flash")
          (Utilities|FlowControl|Delay 0.025)
          (Rendering|Material|SetMaterial (Variables|Default|GetSM_Enemy_Melee_Indicator) 0 "/Game/Enemies/MI_Riot_Shield.MI_Riot_Shield")
          (Utilities|FlowControl|Delay 0.1)
          (Rendering|Material|SetMaterial (Variables|Default|GetSM_Enemy_Melee_Indicator) 0 "/Game/Enemies/M_Enemy_Melee_Indicator_Flash.M_Enemy_Melee_Indicator_Flash"))))))

(fn ConstructionScript)

(fn CanShoot
  (return (Variables|/Game/Weapon/BPC_Weapon.BPC_Weapon_C|GetCan%20Shoot (Variables|Default|GetBPC_Weapon))))

(fn GetAttacking
  (return (Variables|Default|GetAttacking)))

(fn GetEnemyEnum
  (return (.EnemyType (Utilities|Struct|BreakStruct_Enemy_Info (Variables|Default|GetEnemy%20Info)))))

(fn GetEnemyInfo
  (return (Variables|Default|GetEnemy%20Info)))

(fn GetPossessionImmune
  (return (Variables|Default|GetPossession%20Immune)))

(fn GetRiotShield
  (return (Variables|Default|GetRiot%20Shield)))