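; In-game mode Blueprint that runs each timed combat room, tracking game over, score and combo.
; Room start runs the enemy director's spawn loop and timers for the end sound and completion, which deactivates enemies, shows a widget and pauses.
; Player death, bound outside the tutorial, stops spawning and the completion timer.
; Combos multiply score and expire faster as they grow; slow time uses global dilation, pitch and post-processing, optionally compensating the player.
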(event Custom|Room%20Complete
  (if (not (Variables|Default|GetGame%20Over?))
    (Default|CallRoomEnd)
    (bind _returnvalue (Actor|GetActorOfClass "/Game/Enemies/BP_Enemy_Director.BP_Enemy_Director_C"))
    (Default|StopSpawningLoop _returnvalue)
    (bind _outactors (Actor|GetAllActorsOfClass "/Game/Enemies/BP_Enemy.BP_Enemy_C"))
    (for _array_element _outactors
      (Default|DeactivateEnemy _array_element))
    (bind _aspc_player (Utilities|Casting|CastToPC_Player (Game|GetPlayerController 0)))
    (Default|AddRoomCompleteWidget _aspc_player)
    (Game|SetGamePaused true)))

(event Custom|Reset%20Combo
  (bind _output_get (Variables|Default|SetPlayer%20Combo 0))
  (Default|CallComboUpdated _output_get))

(event Custom|Update%20Score
  (params (Add :type Integer))
  (bind _output_get (Variables|Default|SetPlayer%20Score (+ (* Add (+ (Variables|Default|GetPlayer%20Combo) 1)) (Variables|Default|GetPlayer%20Score))))
  (Default|CallScoreUpdated _output_get))

(event Custom|Game%20Over
  (bind _room_end_sound (Variables|Default|GetRoom%20End%20Sound))
  (Variables|Default|SetGame%20Over? true)
  (Utilities|IsValid _room_end_sound
    (:Is%20Valid
      (Audio|Components|Audio|Stop _room_end_sound))
    (:Is%20Not%20Valid
      _))
  (Utilities|FlowControl|Delay 1.6)
  (bind _returnvalue (Actor|GetActorOfClass "/Game/Enemies/BP_Enemy_Director.BP_Enemy_Director_C"))
  (Default|StopSpawningLoop _returnvalue)
  (bind _outactors (Actor|GetAllActorsOfClass "/Game/Enemies/BP_Enemy.BP_Enemy_C"))
  (for _array_element _outactors
    (Default|DeactivateEnemy _array_element))
  (Utilities|Time|ClearandInvalidateTimerbyHandle (Variables|Default|GetRoom%20Complete%20Timer)))

(event Custom|Increment%20Combo
  (Utilities|FlowControl|DoOnce false :!label _label
    (:Completed
      (Utilities|Time|ClearandInvalidateTimerbyHandle (Variables|Default|GetCombo%20Reset%20Timer))
      (bind _result (Math|Integer|IncrementInt (Variables|Default|GetPlayer%20Combo))
        (:%20%20
          (bind _returnvalue (Utilities|Time|SetTimerbyEvent (delegate Custom|Reset%20Combo) (Math|Float|MapRangeClamped (Math|Conversions|ToFloat(Integer) _result) 0.0 15.0 4.0 1.0)))
          (Variables|Default|SetCombo%20Reset%20Timer _returnvalue)
          (Default|CallComboUpdated _result)
          (goto _label Reset))))))

(event Custom|Start%20Room%20End%20Sound
  (bind _returnvalue (Audio|SpawnSound2D "/Game/SFX/Lvl_End.Lvl_End" 1.0 1.0 0.0 0))
  (Variables|Default|SetRoom%20End%20Sound _returnvalue))

(event Custom|Room%20Start
  (Utilities|Time|SetTimerbyEvent (delegate Custom|Start%20Room%20End%20Sound) 57.0)
  (bind _returnvalue (Utilities|Time|SetTimerbyEvent (delegate Custom|Room%20Complete) 6e+01))
  (Variables|Default|SetRoom%20Complete%20Timer _returnvalue)
  (bind _returnvalue_2 (Actor|GetActorOfClass "/Game/Enemies/BP_Enemy_Director.BP_Enemy_Director_C"))
  (Default|StartSpawningLoop _returnvalue_2))

(event EventBeginPlay
  (bind _asbp_game_instance (Utilities|Casting|CastToBP_Game_Instance (Game|GetGameInstance)))
  (Default|BeginMusic _asbp_game_instance)
  (bind _returnvalue (Game|GetCurrentLevelName true))
  (for _index (range 0 (- (|GetNumEnumEntries) 1))
    (if (Utilities|Enum|Equal(Enum) _returnvalue (Utilities|String|EnumtoString (Utilities|Enum|ByteToEnumEnum_Rooms (Math|Conversions|ToByte(Integer) _index))))
      (Variables|Default|SetCurrent%20Room (Utilities|Enum|ByteToEnumEnum_Rooms (Math|Conversions|ToByte(Integer) _index)))))
  (bind _returnvalue_2 (Actor|GetActorOfClass "/Game/Player/BP_Player.BP_Player_C"))
  (Variables|Default|SetPlayer _returnvalue_2)
  (bind _returnvalue_3 (Game|GetCurrentLevelName true))
  (if (not (Utilities|Enum|Equal(Enum) _returnvalue_3 "Tutorial"))
    (Utilities|FlowControl|Delay 0.2)
    (Default|CallRoomStartCountdown)
    (EventDispatchers|BindEventtoPlayerDeath (Actor|GetComponentbyClass (Variables|Default|GetPlayer) "/Game/Player/Components/BPC_Health.BPC_Health_C") (delegate Custom|Game%20Over))))

(fn ConstructionScript)

(fn ActivateSlowTime
  (params (Length :type Float%20%28double-precision%29) (Include%20Player :type Boolean) (Slow%20Time%20Amount :type Float%20%28double-precision%29) (Player%20Specific%20Slow%20Time :type Float%20%28double-precision%29))
  (bind _returnvalue (== Player%20Specific%20Slow%20Time 0.0))
  (bind _player (Variables|Default|GetPlayer))
  (bind _first_person_camera (Variables|/Game/Player/BP_Player.BP_Player_C|GetFirst%20Person%20Camera _player))
  (Utilities|Time|SetTimerbyFunctionName 0 "Deactivate Slow Time" Length)
  (Class|GameplayStatics|SetGlobalPitchModulation Slow%20Time%20Amount 0.5)
  (Utilities|Time|SetGlobalTimeDilation Slow%20Time%20Amount)
  (if Include%20Player
    (bind _structout (Utilities|Struct|SetmembersinPostProcessSettings (Variables|/Script/Engine.CameraComponent|GetPostProcessSettings _first_person_camera) (Math|Float|MapRangeClamped (Math|Float|SelectFloat Slow%20Time%20Amount (stale _output_get) _returnvalue) 0.0 1.0 1.0 0.0) :!label _label))
    (Variables|/Script/Engine.CameraComponent|SetPostProcessSettings _first_person_camera _structout)
    (elif _returnvalue
      (Variables|/Script/Engine.Actor|SetCustomTimeDilation (Variables|Default|GetPlayer) (/ 1.0 Slow%20Time%20Amount))
      (else
        (bind _output_get (Variables|/Script/Engine.Actor|SetCustomTimeDilation (Variables|Default|GetPlayer) Player%20Specific%20Slow%20Time))
        (goto _label)))))

(fn DeactivateSlowTime
  (bind _player (Variables|Default|GetPlayer))
  (bind _first_person_camera (Variables|/Game/Player/BP_Player.BP_Player_C|GetFirst%20Person%20Camera _player))
  (Utilities|Time|SetGlobalTimeDilation 1.0)
  (Class|GameplayStatics|SetGlobalPitchModulation 1.0 0.5)
  (bind _structout (Utilities|Struct|SetmembersinPostProcessSettings (Variables|/Script/Engine.CameraComponent|GetPostProcessSettings _first_person_camera) 0.0))
  (Variables|/Script/Engine.CameraComponent|SetPostProcessSettings _first_person_camera _structout))