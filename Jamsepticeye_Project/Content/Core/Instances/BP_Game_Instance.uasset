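; Game instance that carries run state across levels: score, rooms cleared, player upgrades and persistent background music.
; Room transitions copy the score from the in-game mode, then open a random room, rerolling to avoid repeating the current one.
; Outside that game mode, it opens the tutorial until completed, otherwise a random room.
; A new high score triggers a save of score, tutorial flag, volume and look sensitivity to one slot.
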(event Custom|Transition%20to%20New%20Room
  (Game|SetGamePaused false)
  (bind _asbp_in_game (Utilities|Casting|CastToBP_In_Game (Game|GetGameMode)))
  (Variables|Default|SetCurrent%20Player%20Score (Variables|/Game/Core/Modes/BP_In_Game.BP_In_Game_C|GetPlayer%20Score _asbp_in_game))
  (Math|Integer|IncrementInt (Variables|Default|GetRooms%20Cleared)
    (:%20%20
      (CallFunction|DetermineNextLevel))))

(event Custom|Add%20Upgrade
  (params (Upgrade :type Enum_Upgrades%20Enum :default "NewEnumerator0"))
  (Utilities|Array|Add (Variables|Default|GetCurrent%20Player%20Upgrades) Upgrade))

(event Custom|Reset%20Upgrades
  (Utilities|Array|Clear (Variables|Default|GetCurrent%20Player%20Upgrades)))

(event Custom|Determine%20Highest%20Score
  (if (> (Variables|Default|GetCurrent%20Player%20Score) (Variables|Default|GetCurrent%20Highest%20Score))
    (Variables|Default|SetCurrent%20Highest%20Score (Variables|Default|GetCurrent%20Player%20Score))
    (CallFunction|SaveGame)
    (Variables|Default|SetCurrent%20Player%20Score 0)))

(event Custom|Save%20Game
  (bind _returnvalue (SaveGame|CreateSaveGameObject "/Game/Core/BP_Save_Game.BP_Save_Game_C"))
  (bind _output_get (Variables|Default|SetCreated%20Save%20Game _returnvalue))
  (Variables|/Game/Core/BP_Save_Game.BP_Save_Game_C|SetHighest%20Score _output_get (Variables|Default|GetCurrent%20Highest%20Score))
  (Variables|/Game/Core/BP_Save_Game.BP_Save_Game_C|SetCompleted%20Tutorial _output_get (Variables|Default|GetCompleted%20Tutorial?))
  (Variables|/Game/Core/BP_Save_Game.BP_Save_Game_C|SetMain%20Vol _returnvalue (Variables|Default|GetMain%20Vol))
  (Variables|/Game/Core/BP_Save_Game.BP_Save_Game_C|SetMusic%20Vol _returnvalue (Variables|Default|GetMusic%20Vol))
  (Variables|/Game/Core/BP_Save_Game.BP_Save_Game_C|SetPlayer%20Look%20Sensitivity _returnvalue (Variables|Default|GetPlayer%20Look%20Sensitivity))
  (SaveGame|SaveGametoSlot (Variables|Default|GetCreated%20Save%20Game) "UserSlot"))

(event Custom|Remove%20Upgrade
  (params (Upgrade%20to%20Remove :type Enum_Upgrades%20Enum :default "NewEnumerator0"))
  (Utilities|Array|RemoveItem (Variables|Default|GetCurrent%20Player%20Upgrades) Upgrade%20to%20Remove))

(event Custom|Create%20Game%20Music
  (Utilities|IsValid (Variables|Default|GetIn%20Game%20Music)
    (:Is%20Not%20Valid
      (bind _returnvalue (Audio|SpawnSound2D "/Game/SFX/Music/SC_GameMusic.SC_GameMusic" 1.0 1.0 0.0 0 true false))
      (bind _output_get (Variables|Default|SetIn%20Game%20Music _returnvalue))
      (Class|AudioComponent|SetPaused _output_get true))))

(event Custom|Update%20Play%20Game%20Music
  (params (Playing? :type Boolean))
  (Class|AudioComponent|SetPaused (Variables|Default|GetIn%20Game%20Music) (not Playing?)))

(event Custom|Begin%20Music
  (bind _in_game_music (Variables|Default|GetIn%20Game%20Music))
  (if (Audio|Components|Audio|IsPlaying _in_game_music)
    (Class|AudioComponent|SetPaused _in_game_music false)
    (else
      (Audio|Components|Audio|Play _in_game_music 0.0))))

(fn DetermineNextLevel
  (bind _asbp_in_game (Utilities|Casting|CastToBP_In_Game (Game|GetGameMode))
    (:then
      (if (Utilities|Enum|Equal(Enum) (stale _output_get) (Variables|/Game/Core/Modes/BP_In_Game.BP_In_Game_C|GetCurrent%20Room _asbp_in_game)) :!label _label
        (bind _output_get (Variables|Default|SetTemp%20New%20Room (Utilities|Enum|ByteToEnumEnum_Rooms (Math|Conversions|ToByte(Integer) (Math|Random|RandomIntegerinRange 0 (- (|GetNumEnumEntries) 1))))))
        (goto _label)
        (else
          (Development|PrintString (Utilities|String|EnumtoString (Variables|Default|GetTemp%20New%20Room)))
          (Game|OpenLevel(byObjectReference) (Utilities|Select :Index (Variables|Default|GetTemp%20New%20Room) :NewEnumerator3 "/Game/Core/Maps/Church1.Church1" :NewEnumerator4 "/Game/Core/Maps/Church2.Church2" :NewEnumerator5 "/Game/Core/Maps/CloseQuartersChurch.CloseQuartersChurch" :NewEnumerator6 "/Game/Core/Maps/CloseQuartersChurch2.CloseQuartersChurch2")))))
    (:CastFailed
      (if (Variables|Default|GetCompleted%20Tutorial?)
        (Game|OpenLevel(byObjectReference) (Utilities|Select :Index (Utilities|Enum|ByteToEnumEnum_Rooms (Math|Conversions|ToByte(Integer) (Math|Random|RandomIntegerinRange 0 (- (|GetNumEnumEntries) 1)))) :NewEnumerator3 "/Game/Core/Maps/Church1.Church1" :NewEnumerator4 "/Game/Core/Maps/Church2.Church2" :NewEnumerator5 "/Game/Core/Maps/CloseQuartersChurch.CloseQuartersChurch" :NewEnumerator6 "/Game/Core/Maps/CloseQuartersChurch2.CloseQuartersChurch2"))
        (else
          ;[0 0 0] Open tutorial
          (Game|OpenLevel(byObjectReference) "/Game/Core/Maps/Tutorial.Tutorial"))))))