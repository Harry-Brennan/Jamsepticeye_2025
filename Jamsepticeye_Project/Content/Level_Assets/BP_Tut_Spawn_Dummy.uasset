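; Tutorial trigger that spawns a practice enemy and teaches the player possession and firing.
; The first overlap on PlayerDetection spawns a BP_Enemy at TargetSpawnPoint, flagged as a dummy that stands still, never attacks and has very high health.
; A delayed sequence then swaps the possess hint from a threat to the right-click instruction, deals token damage to the player through BPC_Health and reveals the fire hint.
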(event OnComponentBeginOverlap(PlayerDetection)
  (params (OverlappedComponent :type Primitive%20Component%20Object%20Reference) (OtherActor :type Actor%20Object%20Reference) (OtherComp :type Primitive%20Component%20Object%20Reference) (OtherBodyIndex :type Integer) (bFromSweep :type Boolean) (SweepResult :type Hit%20Result%20Structure%20%28by%20ref%29))
  (Utilities|FlowControl|DoOnce false
    (:Completed
      (CallFunction|SpawnDummy)
      (Utilities|FlowControl|Delay 3.0)
      (Rendering|Components|TextRender|SetText (Variables|/Script/Engine.TextRenderActor|GetTextRender (Variables|Default|GetPossess%20Hint)) (Utilities|Text|MakeLiteralText "IM GOING TO KILL YOU NOW 
GET READY"))
      (Utilities|FlowControl|Delay 3.0)
      (Rendering|Components|TextRender|SetText (Variables|/Script/Engine.TextRenderActor|GetTextRender (Variables|Default|GetPossess%20Hint)) (Utilities|Text|MakeLiteralText "RIGHT CLICK THE ENEMY  
TO POSSESS"))
      (Default|TakeDamage (Actor|GetComponentbyClass (Game|GetPlayerCharacter 0) "/Game/Player/Components/BPC_Health.BPC_Health_C") 1)
      (Utilities|FlowControl|Delay 2.0)
      (Rendering|SetVisibility (Variables|/Script/Engine.TextRenderActor|GetTextRender (Variables|Default|GetFire%20Hint)) true false))))

(event Custom|Spawn%20Dummy
  (bind _target_spawn_point (Variables|Default|GetTarget%20Spawn%20Point))
  (bind _returnvalue (Transformation|GetWorldTransform _target_spawn_point))
  (Game|SpawnActorfromClass "/Game/Enemies/BP_Enemy.BP_Enemy_C" (Math|Transform|MakeTransform (.location _returnvalue) (.rotation _returnvalue) "1.000000,1.000000,1.000000") "Undefined" "MultiplyWithRoot" 0 (Utilities|Struct|MakeStruct_Enemy_Infos "NewEnumerator0" false 0.0 999 0 "NewEnumerator0" 100 1.0 "/Game/Enemies/Sprites/harry_cropped_no_bg_pixelated_Sprite.harry_cropped_no_bg_pixelated_Sprite") true 0))

(fn ConstructionScript)