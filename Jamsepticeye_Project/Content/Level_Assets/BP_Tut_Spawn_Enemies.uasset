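; Tutorial trigger that spawns the final combat wave and ends the tutorial once it is cleared.
; On first box overlap it shows the vanquish-demons text, waits briefly, then spawns and activates enemies at the level's spawn points, mostly melee fodder plus one ranged, using DT_Enemy_Info rows.
; Each death feeds a kill counter; when all are dead it saves completion to the game instance, pauses, and swaps the HUD for the completion widget.
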(event OnComponentBeginOverlap(Box)
  (params (OverlappedComponent :type Primitive%20Component%20Object%20Reference) (OtherActor :type Actor%20Object%20Reference) (OtherComp :type Primitive%20Component%20Object%20Reference) (OtherBodyIndex :type Integer) (bFromSweep :type Boolean) (SweepResult :type Hit%20Result%20Structure%20%28by%20ref%29))
  (Utilities|FlowControl|DoOnce false
    (:Completed
      (Rendering|SetVisibility (Variables|/Script/Engine.TextRenderActor|GetTextRender (Variables|Default|GetVanquish%20Demons%20Text)) true false)
      (Utilities|FlowControl|Delay 3.0)
      (bind _outactors (Actor|GetAllActorsOfClass "/Game/Enemies/BP_Enemy_Spawn_Point.BP_Enemy_Spawn_Point_C"))
      (for _index (range 0 4)
        (bind _returnvalue (Utilities|GetDataTableRow "/Game/Enemies/DT_Enemy_Info.DT_Enemy_Info" (select (== _index 4) "Ranged_Fodder" "Melee_Fodder"))
          (:then
            (bind _returnvalue_2 (Game|SpawnActorfromClass "/Game/Enemies/BP_Enemy.BP_Enemy_C" (Transformation|GetActorTransform (Utilities|Array|Get(acopy) _outactors _index)) "Undefined" "MultiplyWithRoot" 0 _returnvalue false 0))
            (Default|ActivateEnemy _returnvalue_2 _returnvalue (.Location (Math|Transform|BreakTransform (Transformation|GetActorTransform (Utilities|Array|Get(acopy) _outactors _index)))))
            (EventDispatchers|BindEventtoEnemyDeath _returnvalue_2 (delegate Custom|Check%20Tutorial%20Over))))))))

(event Custom|Check%20Tutorial%20Over
  (params (Enemy%20Cost :type Integer) (Enemy%20Score :type Integer))
  (bind _result (Math|Integer|IncrementInt (Variables|Default|GetEnemies%20Killed))
    (:%20%20
      (if (== _result 5)
        (CallFunction|TutorialOver)))))

(event Custom|Tutorial%20Over
  (bind _returnvalue (Game|GetPlayerController 0))
  (bind _asbp_game_instance (Utilities|Casting|CastToBP_Game_Instance (Game|GetGameInstance)))
  (Variables|/Game/Core/Instances/BP_Game_Instance.BP_Game_Instance_C|SetCompleted%20Tutorial? _asbp_game_instance true)
  (Default|SaveGame _asbp_game_instance)
  (Utilities|FlowControl|Delay 1.0)
  (Game|SetGamePaused true)
  (bind _returnvalue_2 (UserInterface|CreateWidget "/Game/UI/WBP_Tutorial_Completed.WBP_Tutorial_Completed_C"))
  (UserInterface|Viewport|AddtoViewport _returnvalue_2 0)
  (Input|SetInputModeUIOnly _returnvalue _returnvalue_2 "DoNotLock" false)
  (Variables|/Script/Engine.PlayerController|SetbShowMouseCursor _returnvalue true)
  (bind _aspc_player (Utilities|Casting|CastToPC_Player (Game|GetPlayerController 0)))
  (Default|RemoveHUD _aspc_player))

(fn ConstructionScript)