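; BP_Moving_Spikes is a spike actor that moves continuously back and forth along a spline path from BeginPlay.
; A timeline maps its DistanceAlongSpline track to the spline's length and sets the actor's world location on each update, without sweeping.
; Its play rate derives from TimeToMove, and each finish re-runs the loop, which plays forward or reverses based on the playback position.
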(event Custom|Moving%20Spikes%20Movement%20Loop
  (Components|Timeline|SetPlayRate (Variables|Default|GetMovement%20Timeline) (/ 1.0 (Variables|Default|GetTime%20to%20Move)))
  (if (== (Components|Timeline|GetPlaybackPosition (Variables|Default|GetMovement%20Timeline)) 0.0)
    (bind ___distance_along_spline (Timeline|Movement%20Timeline PlayFromStart)
      (:Update
        (Transformation|SetActorLocation (Spline|GetLocationatDistanceAlongSpline (Variables|Default|GetMovement%20Spline) (* (Spline|GetSplineLength (Variables|Default|GetMovement%20Spline)) ___distance_along_spline) "World") false false))
      (:Finished
        (CallFunction|MovingSpikesMovementLoop)))
    (else
      (Timeline|Movement%20Timeline ReverseFromEnd))))

(event EventBeginPlay
  (CallFunction|MovingSpikesMovementLoop))

(fn ConstructionScript
  (|CallParentFunction))