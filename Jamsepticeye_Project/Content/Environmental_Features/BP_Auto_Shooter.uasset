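; BP_Auto_Shooter is an environmental shooter that fires a weapon automatically on a repeating timer.
; On BeginPlay it copies its WeaponInfo settings into the BPCWeapon component, fills the ammo to max, and starts a looping timer at the weapon's cooldown interval.
; Each tick of that timer calls the component's fire function from the ShootLoc position, using the SM mesh's world rotation as the aim.
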(event Custom|Auto%20Shooter%20Fire%20Loop
  (Default|FireEquippedWeapon (Variables|Default|GetBPC_Weapon) (Transformation|GetWorldLocation (Variables|Default|GetShoot%20Loc)) (Transformation|GetWorldRotation (Variables|Default|GetSM))))

(event EventBeginPlay
  (bind _weapon_info (Variables|Default|GetWeapon%20Info))
  (bind _bpc_weapon (Variables|Default|GetBPC_Weapon))
  (bind (_enum _projectilespeed _cooldown _lifespan _reloadtime _maxammo _projectilescale) (Utilities|Struct|BreakStruct_Weapons _weapon_info))
  (Variables|/Game/Weapon/BPC_Weapon.BPC_Weapon_C|SetEquipped%20Weapon _bpc_weapon _enum)
  (Variables|/Game/Weapon/BPC_Weapon.BPC_Weapon_C|SetProjectile%20Lifespan _bpc_weapon _lifespan)
  (Variables|/Game/Weapon/BPC_Weapon.BPC_Weapon_C|SetReload%20Time _bpc_weapon _reloadtime)
  (bind _output_get (Variables|/Game/Weapon/BPC_Weapon.BPC_Weapon_C|SetCooldown%20Duration _bpc_weapon _cooldown))
  (Variables|/Game/Weapon/BPC_Weapon.BPC_Weapon_C|SetProjectile%20Speed _bpc_weapon _projectilespeed)
  (bind _output_get_2 (Variables|/Game/Weapon/BPC_Weapon.BPC_Weapon_C|SetMax%20Ammo _bpc_weapon _maxammo))
  (Variables|/Game/Weapon/BPC_Weapon.BPC_Weapon_C|SetCurrent%20Ammo _bpc_weapon _output_get_2)
  (Variables|/Game/Weapon/BPC_Weapon.BPC_Weapon_C|SetProjectile%20Scale _bpc_weapon _projectilescale)
  (bind _returnvalue (Utilities|Time|SetTimerbyEvent (delegate Custom|Auto%20Shooter%20Fire%20Loop) _output_get true))
  (Variables|Default|SetAuto%20Fire%20Timer _returnvalue))

(fn ConstructionScript)