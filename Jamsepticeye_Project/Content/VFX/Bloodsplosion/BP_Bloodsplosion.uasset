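; BP_Bloodsplosion is a short-lived gore effect actor that plays a burst sound and Niagara blood explosion, then destroys itself.
; It passes BloodAmount and itself to Niagara, which returns particle data through the ParticleData callback.
; Each particle spawns a fading decal facing against its velocity, with randomized radius scaled by BloodAmount and one of two dark colours.
; The following splatter sound takes particle velocity, not position, as its location.
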(event EventBeginPlay
  (Audio|PlaySoundatLocation "/Game/VFX/Bloodsplosion/Bloodsplosion_SC.Bloodsplosion_SC" (Transformation|GetActorLocation) "0, 0, 0" 1.0 1.0 0.0 0 0 0 0)
  (Class|NiagaraComponent|SetAsset (Variables|Default|GetBloodSplosion) "/Game/VFX/Bloodsplosion/Niagara/NS_Bloodsplosion.NS_Bloodsplosion" true)
  (Class|NiagaraComponent|SetVariableInt (Variables|Default|GetBloodSplosion) "user.Blood_Amount" (Variables|Default|GetBlood_Amount))
  (Class|NiagaraComponent|SetVariableObject (Variables|Default|GetBloodSplosion) "user.BP_Blood" self)
  (Utilities|FlowControl|Delay 2.2)
  (Actor|DestroyActor))

(event EventParticleData
  (params (Data :type Array%20of%20Basic%20Particle%20Data%20Structures) (NiagaraSystem :type Niagara%20System%20Object%20Reference) (SimulationPositionOffset :type Vector%20%28by%20ref%29 :default "0, 0, 0"))
  (bind _blood_amount (Variables|Default|GetBlood_Amount))
  (for _array_element Data
    (bind _returnvalue (Rendering|Decal|SpawnDecalatLocation "/Game/VFX/Blood_Splatter/Materials/MI_Blood_Decal_Advanced.MI_Blood_Decal_Advanced" "128.000000,256.000000,256.000000" (.Position (Utilities|Struct|BreakBasicParticleData _array_element)) (Math|Conversions|RotationFromXVector (* (.Velocity (Utilities|Struct|BreakBasicParticleData _array_element)) -1.0)) 0.0))
    (Rendering|Components|Decal|SetFadeOut _returnvalue 3.0 5.0 true)
    (bind _returnvalue_2 (Rendering|Material|CreateDynamicMaterialInstance _returnvalue :!class /Script/Engine.DecalComponent))
    (Rendering|Material|SetScalarParameterValue _returnvalue_2 "Radius" (Math|Float|Clamp(Float) (Math|Float|Lerp (* _blood_amount 0.1) (Math|Conversions|ToFloat(Integer) _blood_amount) (Math|Random|RandomFloatinRange 0.0 1.0)) 1.0 3e+02) :!class /Script/Engine.MaterialInstanceDynamic)
    (Rendering|Material|SetVectorParameterValue _returnvalue_2 "Colour" (Math|Color|SelectColor "(R=0.057292,G=0.000000,B=0.000000,A=1.000000)" "(R=0.014789,G=0.000000,B=0.031250,A=1.000000)" (> (Math|Random|RandomFloatinRange 0.0 1.0) 0.25)) :!class /Script/Engine.MaterialInstanceDynamic))
  (Audio|PlaySoundatLocation "/Game/VFX/Blood/Blood_Audio/Blood_Splatter_SC.Blood_Splatter_SC" (.Velocity (Utilities|Struct|BreakBasicParticleData _array_element)) "0, 0, 0" 1.0 1.0 0.0 0 0 0 0))

(fn ConstructionScript)