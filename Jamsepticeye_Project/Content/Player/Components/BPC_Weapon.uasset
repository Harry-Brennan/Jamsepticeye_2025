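; BPC_Weapon is a player weapon component, at an early stage, that fires the currently equipped weapon.
; FireEquippedWeapon prints a debug message and switches on EquippedWeapon, with only the Sniper case wired; its ControlRotation input is unused.
; Sniper sphere-traces from the owner's location along the camera's forward vector against one object type, drawing debug shapes but not yet using the hit.
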(event EventBeginPlay)

(event EventTick
  (params (DeltaSeconds :type Float%20%28single-precision%29)))

(fn FireEquippedWeapon
  (params (Control%20Rotation :type Rotator))
  (Development|PrintString "HOLA AMIGO IT WORKED")
  (switch Utilities|FlowControl|Switch|SwitchonEnum_Weapons (Variables|Default|GetEquipped%20Weapon)
    (:NewEnumerator2
      (|Sniper))))