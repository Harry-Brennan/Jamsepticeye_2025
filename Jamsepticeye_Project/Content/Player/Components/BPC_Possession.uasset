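; Player component for a last-chance possession mechanic: a timed slow-motion window to take over an enemy, or die.
; While active, tick sphere-traces along the view to highlight a non-immune target.
; IA_Possess starts timer-driven FOV and post-process zoom, then moves the player into the enemy's place, copying weapon and speed.
; Possession kills the host, damages nearby enemies, resets health with brief invincibility, and shortens later windows.
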(event Input|EnhancedActionEvents|EnhancedInputActionIA_Possess
  (params (ActionValue :type Boolean) (ElapsedSeconds :type Float%20%28double-precision%29) (TriggeredSeconds :type Float%20%28double-precision%29) (InputAction :type Input%20Action%20Object%20Reference :default "/Game/Player/Input/Actions/IA_Possess.IA_Possess"))
  (if (Variables|Default|GetPossession%20Window%20Active)
    (if (not (Variables|Default|GetAttempting%20Possession))
      (CallFunction|PossessionAttempt))))

(event EventBeginPlay
  (bind _asbp_player (Utilities|Casting|CastToBP_Player (Components|GetOwner)))
  (Variables|Default|SetOwner%20Player _asbp_player))

(event EventTick
  (params (DeltaSeconds :type Float%20%28single-precision%29))
  (bind _returnvalue (Components|GetOwner))
  (bind _returnvalue_2 (Transformation|GetActorLocation _returnvalue))
  (bind (_outhits _returnvalue_3) (Collision|MultiSphereTraceForObjects _returnvalue_2 (+ (* (Math|Vector|GetForwardVector (Pawn|GetControlRotation (Variables|Default|GetOwner%20Player) :!class /Script/Engine.Pawn)) (Variables|Default|GetPossession%20Distance)) _returnvalue_2) (Variables|Default|GetPossession%20Trace%20Radius) (Utilities|Array|MakeArray "ObjectTypeQuery8") false 0 "ForOneFrame"))
  (if _returnvalue_3
    (bind _array_element (Utilities|Array|ForEachLoopwithBreak _outhits :!label _label)
      (:LoopBody
        (Utilities|IsValid (Variables|Default|GetCurrent%20Targeted%20Enemy)
          (:Is%20Valid
            (Class|BPIEnemyMain|DeactivatePossessionIndicator(Message) (Variables|Default|GetCurrent%20Targeted%20Enemy))
            (Variables|Default|SetCurrent%20Targeted%20Enemy 0))
          (:Is%20Not%20Valid
            _))
        (bind _immune_ (Class|BPIEnemyMain|GetPossessionImmune(Message) (.HitActor (Collision|BreakHitResult _array_element))))
        (if (not _immune_)
          (bind _output_get (Variables|Default|SetCurrent%20Targeted%20Enemy (.HitActor (Collision|BreakHitResult _array_element))))
          (Class|BPIEnemyMain|ActivatePossessionIndicator(Message) _output_get)
          (goto _label Break))))
    (else
      (Class|BPIEnemyMain|DeactivatePossessionIndicator(Message) (Variables|Default|GetCurrent%20Targeted%20Enemy))
      (Variables|Default|SetCurrent%20Targeted%20Enemy 0))))

(fn ActivatePossessionWindow
  (bind _owner_player (Variables|Default|GetOwner%20Player))
  (bind _camera_mask (Variables|/Game/Player/BP_Player.BP_Player_C|GetCamera%20Mask _owner_player))
  (if (not (Variables|Default|GetPossession%20Window%20Active))
    (Variables|Default|SetPossession%20Window%20Active true)
    (Variables|Default|SetPossession%20Successful false)
    (bind _returnvalue (Utilities|Time|SetTimerbyFunctionName 0 "Deactivate Possession Window" (Variables|Default|GetPossession%20Window%20Length)))
    (Variables|Default|SetDeactivate%20Possession%20WIndow%20Timer _returnvalue)
    (bind _asbp_in_game (Utilities|Casting|CastToBP_In_Game (Game|GetGameMode)))
    (Default|ActivateSlowTime _asbp_in_game (Variables|Default|GetPossession%20Window%20Length) false 0.5 1.25)
    (Components|Tick|SetComponentTickEnabled true)
    (Default|CallPossessionWindowActiveED)
    (Rendering|Material|SetScalarParameterValue _camera_mask "Radial Colour Amount" 0.55 :!class /Script/Engine.MaterialInstanceDynamic)
    (Rendering|Material|SetVectorParameterValue _camera_mask "Edge Colour" "(R=0.033105,G=0.000000,B=0.165132,A=1.000000)" :!class /Script/Engine.MaterialInstanceDynamic)))

(fn DeactivatePossessionWindow
  (if (Variables|Default|GetAttempting%20Possession)
    (Components|Tick|SetComponentTickEnabled false)
    (Default|CallPossessionWindowDeactivated)
    (else
      (Variables|Default|SetPossession%20Window%20Active false)
      (Components|Tick|SetComponentTickEnabled false)
      (Class|BPIEnemyMain|DeactivatePossessionIndicator(Message) (Variables|Default|GetCurrent%20Targeted%20Enemy))
      (if (Variables|Default|GetPossession%20Successful)
        (Variables|Default|SetCurrent%20Targeted%20Enemy 0)
        (Variables|/Game/Player/Components/BPC_Health.BPC_Health_C|SetAlive (Actor|GetComponentbyClass (Components|GetOwner) "/Game/Player/Components/BPC_Health.BPC_Health_C") true)
        (else
          (Default|Death (Actor|GetComponentbyClass (Components|GetOwner) "/Game/Player/Components/BPC_Health.BPC_Health_C"))
          (Audio|PlaySound2D "/Game/SFX/Death/SC_PlayerDeath.SC_PlayerDeath" 1.0 1.0 0.0 0 0)))
      (Default|CallPossessionWindowDeactivated)
      (Rendering|Material|SetScalarParameterValue (Variables|/Game/Player/BP_Player.BP_Player_C|GetCamera%20Mask (Variables|Default|GetOwner%20Player)) "Radial Colour Amount" 1.0 :!class /Script/Engine.MaterialInstanceDynamic))))

(fn PossessionAttempt
  (bind _current_targeted_enemy (Variables|Default|GetCurrent%20Targeted%20Enemy))
  (Utilities|IsValid _current_targeted_enemy
    (:Is%20Valid
      (Components|Tick|SetComponentTickEnabled false)
      (Variables|Default|SetEnemy%20Location%20for%20Possession (Transformation|GetActorLocation _current_targeted_enemy))
      (Audio|PlaySound2D "/Game/SFX/SC_Possess.SC_Possess" 1.0 1.0 0.0 0 0)
      (CameraShakes|StartCameraShake (Game|GetPlayerCameraManager 0) "/Game/Player/BP_Possession_Attempt_CS.BP_Possession_Attempt_CS_C" 1.0 "CameraLocal" "0, 0, 0")
      (Variables|Default|SetAttempting%20Possession true)
      (Variables|Default|SetZoom%20In? false)
      (bind _returnvalue (Utilities|Time|SetTimerbyFunctionName 0 "Possession Zoom" 0.01 true))
      (Variables|Default|SetPossession%20Zoom%20Timer _returnvalue)
      (bind _returnvalue_2 (Utilities|Time|SetTimerbyFunctionName 0 "Switch Zoom" 0.5))
      (Variables|Default|SetSwitch%20Zoom%20Timer _returnvalue_2)
      (Utilities|Time|SetTimerbyFunctionName 0 "Stop Possession Zoom" 2.0)
      (bind _asbp_in_game (Utilities|Casting|CastToBP_In_Game (Game|GetGameMode)))
      (Default|ActivateSlowTime _asbp_in_game (* (Variables|Default|GetPossession%20Window%20Length) 1.5) false 0.5 1.25))))

(fn PossessionZoom
  (bind _owner_player (Variables|Default|GetOwner%20Player))
  (bind _first_person_camera (Variables|/Game/Player/BP_Player.BP_Player_C|GetFirst%20Person%20Camera _owner_player))
  (Camera|SetFieldOfView _first_person_camera (Math|Interpolation|FInterpTo (Variables|/Script/Engine.CameraComponent|GetFieldOfView (Variables|/Game/Player/BP_Player.BP_Player_C|GetFirst%20Person%20Camera (Variables|Default|GetOwner%20Player))) (Math|Float|SelectFloat 9e+01 1.6e+02 (Variables|Default|GetZoom%20In?)) (Utilities|Time|GetWorldDeltaSeconds) 1e+01))
  (bind _structout (Utilities|Struct|SetmembersinPostProcessSettings (Variables|/Script/Engine.CameraComponent|GetPostProcessSettings _first_person_camera) (Math|Interpolation|FInterpTo (.FilmGrainIntensity (Utilities|Struct|BreakPostProcessSettings (Variables|/Script/Engine.CameraComponent|GetPostProcessSettings _first_person_camera))) (Math|Float|SelectFloat 0.0 1e+01 (Variables|Default|GetZoom%20In?)) (Utilities|Time|GetWorldDeltaSeconds) 12.0) (Math|Interpolation|FInterpTo (.MotionBlurAmount (Utilities|Struct|BreakPostProcessSettings (Variables|/Script/Engine.CameraComponent|GetPostProcessSettings _first_person_camera))) (Math|Float|SelectFloat 0.0 1e+01 (Variables|Default|GetZoom%20In?)) (Utilities|Time|GetWorldDeltaSeconds) 12.0)))
  (Variables|/Script/Engine.CameraComponent|SetPostProcessSettings _first_person_camera _structout))

(fn SwitchZoom
  (Variables|Default|SetZoom%20In? true)
  (CallFunction|UpdatePlayertoPossessedEnemy))

(fn StopPossessionZoom
  (Utilities|Time|ClearandInvalidateTimerbyHandle (Variables|Default|GetPossession%20Zoom%20Timer))
  (Variables|Default|SetAttempting%20Possession false)
  (Variables|Default|SetPossession%20Successful true)
  (CallFunction|DeactivatePossessionWindow))

(fn UpdatePlayertoPossessedEnemy
  (bind _returnvalue (Components|GetOwner))
  (bind _returnvalue_2 (Actor|GetComponentbyClass _returnvalue "/Game/Player/Components/BPC_Health.BPC_Health_C"))
  (bind _enemy_info (Class|BPIEnemyMain|GetEnemyInfo(Message) (Variables|Default|GetCurrent%20Targeted%20Enemy)))
  (Default|SetWeaponInfo (Actor|GetComponentbyClass (Components|GetOwner) "/Game/Weapon/BPC_Weapon.BPC_Weapon_C") (.Weapon (Utilities|Struct|BreakStruct_Enemy_Infos _enemy_info)))
  (Variables|/Script/Engine.CharacterMovementComponent|SetMaxWalkSpeed (Variables|/Script/Engine.Character|GetCharacterMovement (Variables|Default|GetOwner%20Player)) (* 8.5e+02 (.PlayerMoveSpeedOnPossession (Utilities|Struct|BreakStruct_Enemy_Infos _enemy_info))))
  (Transformation|SetActorLocation (Variables|Default|GetOwner%20Player) (Variables|Default|GetEnemy%20Location%20for%20Possession) false false)
  (Pawn|SetControlRotation (Pawn|GetController (Variables|Default|GetOwner%20Player)) (Transformation|GetActorRotation (Variables|Default|GetCurrent%20Targeted%20Enemy)))
  (Default|Death (Actor|GetComponentbyClass (Variables|Default|GetCurrent%20Targeted%20Enemy) "/Game/Player/Components/BPC_Health.BPC_Health_C"))
  (Default|ActivateInvincibility (Actor|GetComponentbyClass (Variables|Default|GetOwner%20Player) "/Game/Player/Components/BPC_Health.BPC_Health_C") 3.0)
  (CallFunction|PossessionAOEKiller)
  (CallFunction|DeactivatePossessionWindow)
  (Variables|/Game/Player/Components/BPC_Health.BPC_Health_C|SetHealth%20Points _returnvalue_2 2)
  (Default|CallPlayerResetHealth _returnvalue_2)
  (bind _result (Math|Integer|IncrementInt (Variables|Default|GetPossessions%20Had%20In%20Lifetime))
    (:%20%20
      (Variables|Default|SetPossession%20Window%20Length (Math|Float|MapRangeClamped (Math|Conversions|ToFloat(Integer) _result) 0.0 8.0 0.75 0.05)))))

(fn PossessionAOEKiller
  (bind _returnvalue (Components|GetOwner))
  (bind _returnvalue_2 (Transformation|GetActorLocation _returnvalue))
  (bind (_outhits _returnvalue_3) (Collision|MultiSphereTraceForObjects _returnvalue_2 _returnvalue_2 6e+02 (Utilities|Array|MakeArray "ObjectTypeQuery8") false 0 "ForDuration"))
  (if _returnvalue_3
    (for _array_element _outhits
      (Default|TakeDamage (Actor|GetComponentbyClass (.HitActor (Collision|BreakHitResult _array_element)) "/Game/Player/Components/BPC_Health.BPC_Health_C") 1))))