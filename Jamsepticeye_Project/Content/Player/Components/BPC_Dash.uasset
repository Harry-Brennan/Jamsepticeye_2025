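; BPC_Dash is an unfinished player dash component that does not yet move anything.
; The Dash event checks CanDash, then tests the IA_Move X input for -1 and, nested inside that, for 1, with no resulting action.
; Unconnected nodes sketch storing the start location and computing an offset from direction or last movement input, along with an unused Lerp.
; Tick is empty.
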(event Custom|Dash
  (bind _returnvalue (Input|EnhancedActionValues|GetIA_Move))
  (bind _x (Math|Vector2D|BreakVector2D _returnvalue))
  (if (Variables|Default|GetCan%20Dash)
    (if (== _x -1.0)
      (if (== _x 1.0)
        _))))

(event EventTick
  (params (DeltaSeconds :type Float%20%28single-precision%29)))