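; Health component shared by the player and enemies, branching on whether the owner implements BPI_Enemy_Main.
; Enemies take max health from that interface and die at zero, while the player starts at a fixed value and opens BPC_Possession's window on a lethal hit.
; Non-lethal player hits trigger timed invincibility, feedback and, with a certain upgrade, sphere-traced damage to nearby health components.
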(event EventBeginPlay
  (if (Utilities|DoesObjectImplementInterface (Components|GetOwner) "/Game/Enemies/BPI_Enemy_Main.BPI_Enemy_Main_C")
    (bind _enemy_info (Class|BPIEnemyMain|GetEnemyInfo(Message) (Components|GetOwner)))
    (Variables|Default|SetHealth%20Points (.EnemyMaxHealth (Utilities|Struct|BreakStruct_Enemy_Infos _enemy_info)))
    (else
      (Variables|Default|SetHealth%20Points 2))))

(event EventTick
  (params (DeltaSeconds :type Float%20%28single-precision%29)))

(fn TakeDamage
  (params (Damage :type Integer))
  (bind _returnvalue (Components|GetOwner))
  (bind _returnvalue_2 (Components|GetOwner))
  (bind _returnvalue_3 (Transformation|GetActorLocation _returnvalue))
  (if (Variables|Default|GetAlive)
    (if (not (Variables|Default|GetInvincible))
      (bind _output_get (Variables|Default|SetHealth%20Points (- (Variables|Default|GetHealth%20Points) Damage)))
      (if (<= _output_get 0)
        (if (Utilities|DoesObjectImplementInterface (Components|GetOwner) "/Game/Enemies/BPI_Enemy_Main.BPI_Enemy_Main_C")
          (CallFunction|Death)
          (Audio|PlaySoundatLocation "/Game/SFX/Death/SC_EnemyDeath.SC_EnemyDeath" "0, 0, 0" "0, 0, 0" 1.0 1.0 0.0 0 0 0 0)
          (else
            (Audio|PlaySound2D "/Game/SFX/SC_PlayerDMG.SC_PlayerDMG" 1.0 1.0 0.0 0 0)
            (Default|ActivatePossessionWindow (Actor|GetComponentbyClass (Components|GetOwner) "/Game/Player/Components/BPC_Possession.BPC_Possession_C"))
            (Variables|Default|SetAlive false)
            (Default|CallPlayerTakeDamage)
            (CameraShakes|StartCameraShake (Game|GetPlayerCameraManager 0) "/Game/Weapon/BP_Shoot_CS.BP_Shoot_CS_C" 5.0 "CameraLocal" "0, 0, 0")))
        (elif (Utilities|DoesObjectImplementInterface _returnvalue_2 "/Game/Enemies/BPI_Enemy_Main.BPI_Enemy_Main_C")
          (Audio|PlaySoundatLocation "/Game/VFX/Blood/Impact_Audio/Impact_SC.Impact_SC" (Transformation|GetActorLocation _returnvalue_2) "0, 0, 0" 1.0 1.0 0.0 0 0 0 0)
          (else
            (Default|CallPlayerTakeDamage)
            (Audio|PlaySound2D "/Game/SFX/SC_PlayerDMG.SC_PlayerDMG" 1.0 1.0 0.0 0 0)
            (CallFunction|ActivateInvincibility 2.0)
            (CameraShakes|StartCameraShake (Game|GetPlayerCameraManager 0) "/Game/Weapon/BP_Shoot_CS.BP_Shoot_CS_C" 5.0 "CameraLocal" "0, 0, 0")
            (bind _asbp_game_instance (Utilities|Casting|CastToBP_Game_Instance (Game|GetGameInstance)))
            (if (Utilities|Array|ContainsItem (Variables|/Game/Core/Instances/BP_Game_Instance.BP_Game_Instance_C|GetCurrent%20Player%20Upgrades _asbp_game_instance) "NewEnumerator9")
              (bind (_outhits _returnvalue_4) (Collision|MultiSphereTraceForObjects _returnvalue_3 _returnvalue_3 256.0 (Utilities|Array|MakeArray "ObjectTypeQuery8") false 0 "None"))
              (if _returnvalue_4
                (for _array_element _outhits
                  (CallFunction|TakeDamage (Actor|GetComponentbyClass (.HitActor (Collision|BreakHitResult _array_element)) "BPC_Health_C") 1))))))))))

(fn Death
  (if (Utilities|DoesObjectImplementInterface (Components|GetOwner) "/Game/Enemies/BPI_Enemy_Main.BPI_Enemy_Main_C")
    (Class|BPIEnemyMain|EnemyDeathEvent(Message) (Components|GetOwner))
    (else
      (Default|CallPlayerDeath))))

(fn ActivateInvincibility
  (params (Invincibility%20Length :type Float%20%28double-precision%29))
  (Variables|Default|SetInvincible true)
  (Utilities|Time|SetTimerbyFunctionName 0 "Deactivate Invincibility" Invincibility%20Length))

(fn DeactivateInvincibility
  (Variables|Default|SetInvincible false))