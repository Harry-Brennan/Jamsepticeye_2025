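; BP_Projectile is a player projectile actor that detects contact with enemies and removes itself after a set lifespan.
; The construction script feeds the Speed variable into the ProjectileMovement component's initial speed, and BeginPlay starts the timed self-destruct.
; Sphere overlaps identify enemies through the BPI_Enemy_Main interface, but a hit only prints a debug string, with no damage or destruction on impact.
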(event OnComponentBeginOverlap(Sphere)
  (params (OverlappedComponent :type Primitive%20Component%20Object%20Reference) (OtherActor :type Actor%20Object%20Reference) (OtherComp :type Primitive%20Component%20Object%20Reference) (OtherBodyIndex :type Integer) (bFromSweep :type Boolean) (SweepResult :type Hit%20Result%20Structure%20%28by%20ref%29))
  (if (Utilities|DoesObjectImplementInterface OtherActor "/Game/Enemies/BPI_Enemy_Main.BPI_Enemy_Main_C")
    (Development|PrintString "yeah")))

(event EventBeginPlay
  (Utilities|FlowControl|Delay (Variables|Default|GetLifespan))
  (Actor|DestroyActor))

(event Collision|EventActorBeginOverlap
  (params (OtherActor :type Actor%20Object%20Reference)))

(event EventTick
  (params (DeltaSeconds :type Float%20%28single-precision%29)))

(fn ConstructionScript
  (Variables|/Script/Engine.ProjectileMovementComponent|SetInitialSpeed (Variables|Default|GetProjectileMovement) (Variables|Default|GetSpeed)))